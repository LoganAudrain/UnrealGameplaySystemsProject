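; AI agent Blueprint that links a weapon-wielding enemy to its AI controller's Blackboard, extending a parent class that holds migrated logic.
; BeginPlay seeds full health, binds weapon action-stopped and ammo-changed events, then reloads; attack and reload events forward to the weapon.
; Handlers write health and ammo to Blackboard keys and send an AI message when an action finishes.
; The construction script tints the mesh materials with the agent's color.
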(event `self.ReceiveTick`
  (params (DeltaSeconds :type "Float (single-precision)"))
  ;[1 1 1] Migrated to code
  (`parent.ReceiveTick` 0.0))

(event `self.ReceiveBeginPlay`
  ;[1 1 1] Gar - Week 1
  (`parent.ReceiveBeginPlay`)
  (add `/Game/Blueprints/Actors/BP_BaseRifle.OnActionStopped` (`self.WeaponObject`) (`|CreateDelegate` :!event `Handle Action Finished`))
  (`self.UpdateBlackboardHealth` 1.0)
  ;[1 1 1] gar - week 2
  (add `/Game/Blueprints/Actors/BP_BaseRifle.OnAmmoChanged` (`self.WeaponObject`) (`|CreateDelegate` :!event `UpdateBlackboardAmmo`))
  (`/Game/Blueprints/Actors/BP_BaseRifle.ReloadAmmo` (`self.WeaponObject`)))

(event `/Game/Blueprints/Utility/BI_EnemyInterface.EnemyAttack`
  ;[1 1 1] Gar - Week 1
  (`/Game/Blueprints/Actors/BP_BaseRifle.Attack` (`self.WeaponObject`)))

(event `/Game/Blueprints/Utility/BI_EnemyInterface.EnemyReload`
  ;[1 1 1] Gar - week 2
  (`/Game/Blueprints/Actors/BP_BaseRifle.RequestReload` (`self.WeaponObject`)))

(fn `Handle Action Finished`
  (`AIBlueprintHelperLibrary.SendAIMessage` self (`self.ActionFinishedMsg`)))

(fn `Handle Hurt`
  (params (Ratio :type "Float (double-precision)"))
  (`parent.Handle Hurt` Ratio)
  (`self.UpdateBlackboardHealth` Ratio))

(fn `UpdateBlackboardAmmo`
  (params (Current :type "Float (double-precision)") (Max :type "Float (double-precision)"))
  ;[1 1 1] Gar - Week 2
  (`BlackboardComponent.SetValueAsFloat` (`AIBlueprintHelperLibrary.GetBlackboard` (`AIBlueprintHelperLibrary.GetAIController` self)) (`self.AmmoKey`) Current))

(fn `UpdateBlackboardHealth`
  (params (ratio :type "Float (double-precision)"))
  (`BlackboardComponent.SetValueAsFloat` (`AIBlueprintHelperLibrary.GetBlackboard` (`AIBlueprintHelperLibrary.GetAIController` self)) (`self.HealthKey`) ratio))

(fn `UserConstructionScript`
  ;[1 1 1] Migrated to code
  (`parent.UserConstructionScript`)
  (`MeshComponent.SetVectorParameterValueOnMaterials` (`self.Mesh`) (`self.TintName`) (`KismetMathLibrary.Conv_LinearColorToVector` (`self.Color`))))