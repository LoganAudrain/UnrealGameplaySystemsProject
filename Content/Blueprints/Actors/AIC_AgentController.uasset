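; AI controller for agents that runs a behavior tree when it possesses a pawn.
; The construction script binds an event to the AI Perception component's target update.
; The perception handler writes the sensed actor to the player blackboard key, or clears that key when sensing fails.
; It applies no filter on which actor was sensed.
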(event `self.ReceivePossess`
  (params (PossessedPawn :type "Pawn Object Reference"))
  ;[1 1 1] Gar - Week 1
  (`parent.ReceivePossess` PossessedPawn)
  (`self.RunBehaviorTree` (`self.BTAsset`)))

(fn `Handle Perception`
  (params (Actor :type "Actor Object Reference") (Stimulus :type "AIStimulus Structure"))
  (bind _blackboard (`self.Blackboard`))
  (bind _playerkey (`self.PlayerKey`))
  ;[1 1 1] Gar - Week 1
  (if (`.bSuccessfullySensed` (break `AIStimulus` Stimulus))
    (`BlackboardComponent.SetValueAsObject` _blackboard _playerkey Actor)
    (else
      (`BlackboardComponent.ClearValue` _blackboard _playerkey))))

(fn `UserConstructionScript`
  ;[1 1 1] Gar - Week 1
  (add `AIPerceptionComponent.OnTargetPerceptionUpdated` (`self.AIPerception`) (`|CreateDelegate` :!event `Handle Perception`)))