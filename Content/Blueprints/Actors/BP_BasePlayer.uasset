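; Base player Blueprint that handles movement, look, attack and reload input, and always allows health pickups.
; Movement follows control yaw only, while attack and reload are forwarded to WeaponObject.
; BeginPlay creates the HUD, binds health hurt, death and heal events plus weapon ammo changes, and fills ammo.
; Without a PlayerController it prints an error and destroys itself.
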(event `InputAxis|TurnRight`
  (params (AxisValue :type "Float (single-precision)"))
  ;[1 1 1] Week 2 or before
  (`self.AddControllerYawInput` AxisValue))

(event `InputAxis|LookUp`
  (params (AxisValue :type "Float (single-precision)"))
  ;[1 1 1] Week 2 or before
  (`self.AddControllerPitchInput` AxisValue))

(event `InputAxis|MoveForward`
  (params (AxisValue :type "Float (single-precision)"))
  ;[1 1 1] Week 2 or before
  (`self.AddMovementInput` (`KismetMathLibrary.GetForwardVector` (`KismetMathLibrary.MakeRotator` 0.0 0.0 (.yaw (`self.GetControlRotation`)))) AxisValue))

(event `InputAxis|Strafe`
  (params (AxisValue :type "Float (single-precision)"))
  ;[1 1 1] Week 2 or before
  (`self.AddMovementInput` (`KismetMathLibrary.GetRightVector` (`KismetMathLibrary.MakeRotator` 0.0 0.0 (.yaw (`self.GetControlRotation`)))) AxisValue))

(event `InputAction|AttackInput`
  (params (Key :type "Key Structure"))
  ;[1 1 1] Week 2 or before
  (:`Pressed`
    (`/Game/Blueprints/Actors/BP_BaseRifle.Attack` (`self.WeaponObject`))))

(event `InputAction|Reload`
  (params (Key :type "Key Structure"))
  ;[1 1 1] Gar - week 2
  (:`Pressed`
    (`/Game/Blueprints/Actors/BP_BaseRifle.RequestReload` (`self.WeaponObject`))))

(event `self.ReceiveBeginPlay`
  (bind _healthcomponent (`self.HealthComponent`))
  ;[1 1 1] Migrated to Code
  (`parent.ReceiveBeginPlay`)
  (bind _asplayer_controller (cast `PlayerController` (`self.GetController`))
    (:`then`
      (bind _returnvalue (`|CreateWidget` (`self.HUDClass`) _asplayer_controller))
      (bind _output_get (set `self.PlayerHud` _returnvalue))
      (`UserWidget.AddToViewport` _output_get 0)
      (add `/Game/Blueprints/Utility/AC_HealthComponent.OnHurt` _healthcomponent (`|CreateDelegate` (`self.PlayerHud`) :!event `SetHealth`))
      (add `/Game/Blueprints/Utility/AC_HealthComponent.OnDeath` _healthcomponent (`|CreateDelegate` (`self.PlayerHud`) :!event `SetHealth`))
      ;[1 1 1] Gar - Week 2
      (add `/Game/Blueprints/Actors/BP_BaseRifle.OnAmmoChanged` (`self.WeaponObject`) (`|CreateDelegate` (`self.PlayerHud`) :!event `SetAmmo`))
      (`/Game/Blueprints/Actors/BP_BaseRifle.ReloadAmmo` (`self.WeaponObject`))
      (add `/Game/Blueprints/Utility/AC_HealthComponent.OnHeal` (`self.HealthComponent`) (`|CreateDelegate` (`self.PlayerHud`) :!event `SetHealth`)))
    (:`CastFailed`
      (`KismetSystemLibrary.PrintString` "Failed to cast to player controller when creating the hud")
      (`self.K2_DestroyActor`))))

(fn `CanPickupHealth`
  (returns (Yes :type Boolean))
  (return true))

(fn `UserConstructionScript`
  (`parent.UserConstructionScript`))