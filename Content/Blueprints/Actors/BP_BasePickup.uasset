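; Base pickup actor that reacts when another actor overlaps its BoxCollision, with the overlap delegate bound in the Construction Script.
; The overlap handler runs a template-method chain: CanPickup gates HandlePickup, then PostPickup follows.
; By default CanPickup accepts any actor, HandlePickup is an empty hook for the pickup effect, and PostPickup destroys the actor.
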(fn `Bound Overlap`
  (params (OverlappedComponent :type "PrimitiveComponent Object Reference") (OtherActor :type "Actor Object Reference") (OtherComp :type "PrimitiveComponent Object Reference") (OtherBodyIndex :type Integer) (bFromSweep :type Boolean) (SweepResult :type "HitResult Structure (by ref)"))
  ;[1 1 1] GAR - Week 2
  (if (`self.CanPickup` OtherActor)
    (`self.HandlePickup` OtherActor SweepResult)
    (`self.PostPickup`)
    (return)))

(fn `CanPickup`
  (params (OtherActor :type "Actor Object Reference"))
  (returns (Yes :type Boolean))
  ;[1 1 1] Gar - week 2
  (return true))

(fn `HandlePickup`
  (params (OtherActor :type "Actor Object Reference") (SweepResult :type "HitResult Structure")))

(fn `PostPickup`
  ;[1 1 1] Gar - week 2
  (`self.K2_DestroyActor`))

(fn `UserConstructionScript`
  ;[1 1 1] Gar - week 2
  (add `PrimitiveComponent.OnComponentBeginOverlap` (`self.BoxCollision`) (`|CreateDelegate` :!event `Bound Overlap`)))