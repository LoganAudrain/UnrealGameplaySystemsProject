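; Base rifle actor, attached to a parent pawn, that fires projectiles from a weapon socket and tracks ammo.
; Attack spawns a projectile when loaded and idle, spends a round and sets a busy flag with a reset timer.
; Dispatchers announce attacks, reload starts, finished actions and ammo changes; RequestReload only flags and announces, while ReloadAmmo refills.
; An aim hack points player shots at the HUD widget's destination, while agents use base aim rotation.
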(event `self.ReceiveBeginPlay`
  ;[1 1 1] Migrated to code
  (`parent.ReceiveBeginPlay`)
  (bind _aspawn (cast `Pawn` (`self.GetParentActor`))
    (:`then`
      (set `self.Parent Pawn` _aspawn)
      ;[1 1 1] Gar - Week 2
      (`self.ReloadAmmo`))
    (:`CastFailed`
      (`KismetSystemLibrary.PrintString` "Owner must be a pawn")
      (`self.K2_DestroyActor`))))

(event `ActionStopped`
  ;[1 1 1] Gar - Week1
  (set `self.ActionHappening` false)
  (`self.OnActionStopped`))

(event `ReloadAmmo`
  (bind _maxammo (`self.MaxAmmo`))
  ;[1 1 1] Gar - Week 2
  (bind _output_get (set `self.CurrentAmmo` _maxammo))
  (`self.OnAmmoChanged` _output_get _maxammo))

(fn `Attack`
  (bind _parent_pawn (`self.Parent Pawn`))
  ;[1 1 1] Week 2
  (if (`self.CanShoot`)
    (`|SpawnActorFromClass` (`self.Projectile Class`) (`KismetMathLibrary.MakeTransform` (`self.GetSource`) (`self.HACK_DO_NOT_EXPOSE_TO_CODE`)) "Undefined" "MultiplyWithRoot" (`Pawn.GetController` _parent_pawn) _parent_pawn)
    (set `self.ActionHappening` true)
    (`KismetSystemLibrary.K2_SetTimerDelegate` (`|CreateDelegate` :!event `ActionStopped`) (`self.ResetTime`))
    (`self.OnRifleAttack`)
    ;[1 1 1] Gar - Week 2
    (`self.UseAmmo`)))

(fn `CanShoot`
  (returns (Yes :type Boolean))
  ;[1 1 1] END
  (return (and (not (`self.ActionHappening`)) (> (`self.CurrentAmmo`) 0.0))))

(fn `GetSource`
  (returns (ReturnValue :type "Vector Structure"))
  (return (`SceneComponent.GetSocketLocation` (`self.SkeletalMesh`) (`self.WeaponSocketName`))))

(fn `HACK_DO_NOT_EXPOSE_TO_CODE`
  (returns (Rotation :type "Rotator Structure"))
  ;[1 1 1] Checks to see if it is a player or agent
  (bind _foundwidgets (`WidgetBlueprintLibrary.GetAllWidgetsOfClass` "/Game/Both/WBP_PlayerHud.WBP_PlayerHud_C" false))
  (bind _output (`|GetArrayItem` _foundwidgets))
  (if (== (`UserWidget.GetOwningPlayerPawn` _output) (`self.Parent Pawn`))
    ;[1 1 1] Player override get base aim rotation
    (return (`KismetMathLibrary.MakeRotFromX` (- (`PlayerHud.GetDestination` _output) (`self.GetSource`))))
    (else
      ;[1 1 1] This is the agent, do not need to override function
      (return (`Pawn.GetBaseAimRotation` (`self.Parent Pawn`))))))

(fn `RequestReload`
  ;[1 1 1] Gar - week 2
  (if (not (`self.ActionHappening`))
    (set `self.ActionHappening` true)
    (`self.OnReloadStart`)))

(fn `UseAmmo`
  ;[1 1 1] Gar - Week 2
  (bind _output_get (set `self.CurrentAmmo` (`KismetMathLibrary.FMax` (- (`self.CurrentAmmo`) 1.0))))
  (`self.OnAmmoChanged` _output_get (`self.MaxAmmo`)))

(fn `UserConstructionScript`)