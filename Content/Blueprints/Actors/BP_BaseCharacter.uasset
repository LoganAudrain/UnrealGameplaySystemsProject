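; Base character Blueprint that spawns a rifle and wires it to the animation Blueprint and health component, with comments marking logic as migrated to code.
; BeginPlay sets the weapon class on a child actor, destroying the character if the rifle or animation casts fail.
; It then binds attack, hurt and reload delegates.
; HandleHurt forwards a ratio to the hit animation, and CanPickupHealth returns false.
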(event `self.ReceiveBeginPlay`
  (bind _childactorcomponent (`self.ChildActorComponent`))
  ;[1 1 1] Migrated to code
  (`parent.ReceiveBeginPlay`)
  (`ChildActorComponent.SetChildActorClass` _childactorcomponent (`self.Weapon Class`))
  (bind _asbp_base_rifle (cast `/Game/Blueprints/Actors/BP_BaseRifle` (`ChildActorComponent.ChildActor` _childactorcomponent))
    (:`then`
      (set `self.WeaponObject` _asbp_base_rifle)
      (bind _asabp_character_animation (cast `/Game/Both/ABP_CharacterAnimation` (`SkeletalMeshComponent.GetAnimInstance` (`self.Mesh`)))
        (:`then`
          (set `self.AnimationBP` _asabp_character_animation)
          (add `/Game/Blueprints/Actors/BP_BaseRifle.OnRifleAttack` (`self.WeaponObject`) (`|CreateDelegate` (`self.AnimationBP`) :!event `FireAnimation`))
          (add `/Game/Blueprints/Utility/AC_HealthComponent.OnHurt` (`self.HealthComponent`) (`|CreateDelegate` :!event `Handle Hurt`))
          ;[1 1 1] Gar - Week 2
          (add `CharacterAnimation.OnReloadEnded` (`self.AnimationBP`) (`|CreateDelegate` (`self.WeaponObject`) :!event `ActionStopped`))
          (add `CharacterAnimation.OnReloadNow` (`self.AnimationBP`) (`|CreateDelegate` (`self.WeaponObject`) :!event `ReloadAmmo`))
          (add `/Game/Blueprints/Actors/BP_BaseRifle.OnReloadStart` (`self.WeaponObject`) (`|CreateDelegate` (`self.AnimationBP`) :!event `ReloadAnimation`)))
        (:`CastFailed`
          (`KismetSystemLibrary.PrintString` "Needs another anim blueprint")
          (`self.K2_DestroyActor`))))
    (:`CastFailed`
      (`KismetSystemLibrary.PrintString` "<ERROR> No weapon selected")
      (`self.K2_DestroyActor`))))

(fn `CanPickupHealth`
  (returns (Yes :type Boolean))
  ;[1 1 1] Gar - Week 2
  (return false))

(fn `Handle Hurt`
  (params (Ratio :type "Float (double-precision)"))
  ;[1 1 1] Moved to code
  (`CharacterAnimation.HitAnimation` (`self.AnimationBP`) Ratio))

(fn `UserConstructionScript`)