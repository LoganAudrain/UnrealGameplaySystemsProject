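; BP_Projectile is a projectile actor that damages whatever overlaps its sphere collision, then destroys itself.
; The construction script scales the sphere and binds its overlap event, and HandleOverlap applies Damage credited to the owning controller.
; BeginPlay calls the parent, starts a one-shot DestroyTime timer and caches the owner as a Controller, printing on cast failure.
; Comments mark the construction script and HandleOverlap as migrated to code.
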(event `self.ReceiveBeginPlay`
  ;[1 1 1] Week 2 and before
  (`parent.ReceiveBeginPlay`)
  (`KismetSystemLibrary.K2_SetTimerDelegate` (`|CreateDelegate` :!event `K2_DestroyActor`) (`self.DestroyTime`))
  (bind _ascontroller (cast `Controller` (`self.GetOwner`))
    (:`then`
      (set `self.OwnerController` _ascontroller))
    (:`CastFailed`
      (`KismetSystemLibrary.PrintString` "Failed to cast to controller"))))

(fn `HandleOverlap`
  (params (OverlappedComponent :type "PrimitiveComponent Object Reference") (OtherActor :type "Actor Object Reference") (OtherComp :type "PrimitiveComponent Object Reference") (OtherBodyIndex :type Integer) (bFromSweep :type Boolean) (SweepResult :type "HitResult Structure (by ref)"))
  ;[1 1 1] Migrated to Code
  (`GameplayStatics.ApplyDamage` OtherActor (`self.Damage`) (`self.OwnerController`) self)
  (`self.K2_DestroyActor`)
  (return))

(fn `UserConstructionScript`
  ;[1 1 1] Migrated to Code
  (add `PrimitiveComponent.OnComponentBeginOverlap` (`self.Sphere Collision`) (`|CreateDelegate` :!event `HandleOverlap`))
  (`SceneComponent.SetWorldScale3D` (`self.Sphere Collision`) (`self.Scale`)))